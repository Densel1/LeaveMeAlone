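; GM_LMA is the game mode for LeaveMeAlone that runs a one-minute countdown and ends play when time runs out.
; BeginPlay sets GameTime and starts a looping one-second timer that decrements it.
; At zero it clears the timer, shows the WBP_TimeOver widget and switches the PC_LMA controller to UI-only input focused on that widget.
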(event Custom|CustomEvent
  (bind _output_get (Variables|Default|SetGameTime (- (Variables|Default|GetGameTime) 1)))
  (if (== _output_get 0)
    (Utilities|Time|ClearandInvalidateTimerbyHandle (Variables|Default|GetHendlerTimer))
    (bind _returnvalue (UserInterface|CreateWidget "/Game/LeaveMeAlone/Widgets/UI/WBP_TimeOver.WBP_TimeOver_C"))
    (UserInterface|Viewport|AddtoViewport _returnvalue 0)
    (bind _aspc_lma (Utilities|Casting|CastToPC_LMA (Game|GetPlayerController 0)))
    (Input|SetInputModeUIOnly _aspc_lma _returnvalue "DoNotLock" false)))

(event EventBeginPlay
  (Variables|Default|SetGameTime 60)
  (bind _returnvalue (Utilities|Time|SetTimerbyEvent (delegate Custom|CustomEvent) 1.0 true))
  (Variables|Default|SetHendlerTimer _returnvalue))

(event EventTick
  (params (DeltaSeconds :type Float%20%28single-precision%29)))

(fn ConstructionScript)